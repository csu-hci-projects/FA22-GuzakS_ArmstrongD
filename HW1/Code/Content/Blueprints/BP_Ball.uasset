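; BP_Ball is the ball actor in Speedball, tracking its health and handling its own destruction.
; ReduceHealth subtracts damage scaled by the game instance's Difficulty and destroys the ball when Health runs out, while FellOffMap destroys it immediately.
; On Destroyed, it passes itself to GM_Speedball's PlayerRespawn, so the game mode handles respawning.
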(event `self.ReceiveDestroyed`
  (bind _asgm_speedball (cast `/Game/Blueprints/GM_Speedball` (`GameplayStatics.GetGameMode`)))
  (`/Game/Blueprints/GM_Speedball.Player Respawn` _asgm_speedball self))

(fn `FellOffMap`
  (`self.K2_DestroyActor`))

(fn `GetBallRef`
  (returns (Ball :type "/Game/Blueprints/BP_Ball Object Reference"))
  (return self))

(fn `GetBallRef2`
  (returns (BPBall2 :type "/Game/Blueprints/BP_Ball Object Reference"))
  (return null))

(fn `ReduceHealth`
  (bind _asspeedball_instance (cast `/Game/Blueprints/Speedball_Instance` (`GameplayStatics.GetGameInstance`)))
  (bind _output_get (set `self.Health` (- (`self.Health`) (* (`/Game/Blueprints/Speedball_Instance.Difficulty` _asspeedball_instance) 15))))
  (if (<= _output_get 0)
    (`self.K2_DestroyActor`)))

(fn `UserConstructionScript`)