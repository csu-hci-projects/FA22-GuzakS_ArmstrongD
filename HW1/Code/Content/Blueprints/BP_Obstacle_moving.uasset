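; Moving obstacle actor that damages the player's ball on overlap.
; Tick translates it along a normalized Direction at Speed without sweeping, while a looping timer started at BeginPlay flips Direction every TimeToChange seconds for back-and-forth motion.
; Any actor overlap plays a sound at the world origin, then calls ReduceHealth on the player pawn if it is a BP_Ball, without checking which actor overlapped.
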(event `self.ReceiveActorBeginOverlap`
  (params (OtherActor :type "Actor Object Reference"))
  (`GameplayStatics.PlaySoundAtLocation` "/Engine/EditorSounds/Notifications/CompileFailed.CompileFailed" (0.0 0.0 0.0) (struct) 1.0 1.0 0.0 null null null null)
  (bind _asbp_ball (cast `/Game/Blueprints/BP_Ball` (`GameplayStatics.GetPlayerPawn` 0)))
  (`/Game/Blueprints/BP_Ball.ReduceHealth` _asbp_ball))

(event `self.ReceiveTick`
  (params (DeltaSeconds :type "Float (single-precision)"))
  (`self.K2_AddActorWorldOffset` (* (`KismetMathLibrary.Normal` (`self.direction`)) (* (`self.speed`) (`GameplayStatics.GetWorldDeltaSeconds`)))))

(event `self.ReceiveBeginPlay`
  (`KismetSystemLibrary.K2_SetTimerDelegate` (delegate `Change Direction`) (`self.timeToChange`) true))

(event `Change Direction`
  (set `self.direction` (* (`self.direction`) -1.0)))

(fn `UserConstructionScript`)