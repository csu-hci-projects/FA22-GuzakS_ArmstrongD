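; Speedball game mode that handles lives, respawning, the HUD and end-of-level score for the player's ball.
; BeginPlay stores the starting pawn transform as the respawn point and shows the HUD after a short delay.
; PlayerRespawn spends a life and spawns a new pawn, then either possesses it or, at zero lives, resets the game instance score, stops sound and shows the OOL widget.
; CalcScore adds ball health and a spare-life bonus to that score.
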(event `Player Respawn`
  (params (player :type "/Game/Blueprints/BP_Ball Object Reference"))
  (bind _output_get (set `self.Lives` (- (`self.Lives`) 1)))
  (bind _returnvalue (`|SpawnActorFromClass` (`GameplayStatics.GetObjectClass` player) (`self.Respawn location`) "Undefined" "OverrideRootScale" null null))
  (if (<= _output_get 0)
    (`GameplayStatics.SetGamePaused` false)
    (set `PlayerController.bShowMouseCursor` true (`GameplayStatics.GetPlayerController` 0))
    (`WidgetLayoutLibrary.RemoveAllWidgets`)
    (bind _asspeedball_instance (cast `/Game/Blueprints/Speedball_Instance` (`GameplayStatics.GetGameInstance`)))
    (set `/Game/Blueprints/Speedball_Instance.Score` 0 _asspeedball_instance)
    (bind _returnvalue_2 (`|CreateWidget` "/Game/Blueprints/Interfaces/OOL.OOL_C"))
    (`UserWidget.AddToViewport` _returnvalue_2 0)
    (bind _asspeedball_instance_2 (cast `/Game/Blueprints/Speedball_Instance` (`GameplayStatics.GetGameInstance`)))
    (`/Game/Blueprints/Speedball_Instance.stop sound` _asspeedball_instance_2)
    (else
      (`Controller.Possess` (`GameplayStatics.GetPlayerController` 0) _returnvalue))))

(event `self.ReceiveBeginPlay`
  (set `self.Respawn location` (`self.GetTransform` (`GameplayStatics.GetPlayerPawn` 0)))
  (`KismetSystemLibrary.Delay` 0.2)
  (bind _returnvalue (`|CreateWidget` "/Game/Blueprints/Interfaces/HUD.HUD_C"))
  (`UserWidget.AddToViewport` _returnvalue 0))

(fn `calc_score`
  (bind _asbp_ball (cast `/Game/Blueprints/BP_Ball` (`GameplayStatics.GetPlayerPawn` 0)))
  (bind _asspeedball_instance (cast `/Game/Blueprints/Speedball_Instance` (`GameplayStatics.GetGameInstance`)))
  (set `/Game/Blueprints/Speedball_Instance.Score` (+ (`/Game/Blueprints/Speedball_Instance.Score` _asspeedball_instance) (+ (`/Game/Blueprints/BP_Ball.Health` _asbp_ball) (* (- (`self.Lives`) 1) 100))) _asspeedball_instance))

(fn `UserConstructionScript`)